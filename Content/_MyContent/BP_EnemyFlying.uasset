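; BP_EnemyFlying is an enemy that spins its firing rig and shoots while any actor overlaps it.
; Overlap toggles InRange, which Tick uses to play or stop the yaw Timeline.
; The Timeline triggers Shoot once, starting a looping timer that spawns bullets from two firing points whenever InRange is true.
; On hitting the third-person character, it launches them against their velocity and destroys itself.
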(event Custom|Shoot
  (if (Variables|Default|GetInRange)
    (Variables|Default|SetIsShooting true)
    (Utilities|Time|SetTimerbyEvent (delegate Custom|Shoot) (Variables|Default|GetFiringRate) true)
    (CallFunction|DoubleFire)))

(event Custom|Rotate
  (if (Variables|Default|GetInRange)
    _))

(event EventBeginPlay)

(event Collision|EventActorBeginOverlap
  (params (OtherActor :type Actor%20Object%20Reference))
  (Variables|Default|SetInRange true))

(event EventTick
  (params (DeltaSeconds :type Float%20%28single-precision%29))
  (if (Variables|Default|GetInRange)
    (bind _firingr (Timeline|Timeline Play)
      (:Update
        _)
      (:Finished
        _))
    (Transformation|SetRelativeRotation (Variables|Default|GetSM_FiringR) (Math|Rotator|MakeRotator 0.0 0.0 _firingr) false false)
    (if (not (Variables|Default|GetIsShooting))
      (CallFunction|Shoot))
    (else
      (Timeline|Timeline Stop))))

(event Collision|EventActorEndOverlap
  (params (OtherActor :type Actor%20Object%20Reference))
  (Variables|Default|SetInRange false))

(event Collision|EventHit
  (params (MyComp :type Primitive%20Component%20Object%20Reference) (Other :type Actor%20Object%20Reference) (OtherComp :type Primitive%20Component%20Object%20Reference) (bSelfMoved :type Boolean) (HitLocation :type Vector :default "0, 0, 0") (HitNormal :type Vector :default "0, 0, 0") (NormalImpulse :type Vector :default "0, 0, 0") (Hit :type Hit%20Result%20Structure%20%28by%20ref%29))
  (bind _asbp_third_person_character (Utilities|Casting|CastToBP_ThirdPersonCharacter Other))
  (Character|LaunchCharacter _asbp_third_person_character (* (Transformation|GetVelocity _asbp_third_person_character) -3.0) false false)
  (Actor|DestroyActor))

(fn ConstructionScript)

(fn DoubleFire
  (bind _sm_firingpoint1 (Variables|Default|GetSM_FiringPoint1))
  (bind _sm_firingpoint2 (Variables|Default|GetSM_FiringPoint2))
  (bind _returnvalue (Transformation|GetSocketTransform _sm_firingpoint1 "None" "RTS_World"))
  (bind _returnvalue_2 (Transformation|GetSocketTransform _sm_firingpoint2 "None" "RTS_World"))
  (Game|SpawnActorfromClass "/Game/_MyContent/BP_EnemyBullet.BP_EnemyBullet_C" (Math|Transform|MakeTransform (.location _returnvalue) (.rotation _returnvalue) "1.000000,1.000000,1.000000") "Undefined" "MultiplyWithRoot" 0 0)
  (Game|SpawnActorfromClass "/Game/_MyContent/BP_EnemyBullet.BP_EnemyBullet_C" (Math|Transform|MakeTransform (.location _returnvalue_2) (.rotation _returnvalue_2) "1.000000,1.000000,1.000000") "Undefined" "MultiplyWithRoot" 0 0))