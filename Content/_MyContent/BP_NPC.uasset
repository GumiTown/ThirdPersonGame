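; BP_NPC is a dialogue NPC that shows the player's dialogue HUD while an actor tagged Player overlaps it.
; Overlap begin and end toggle InRange and call BP_ThirdPersonCharacter to create or delete that HUD.
; UpdateDialogue copies the current Dialogue array entry into the character's CurrentDialogueText and advances the index without a bounds check.
; ResetDialogue jumps to a hardcoded index before updating.
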(event Custom|UpdateDialogue
  ;[0.07812 0.07812 0.07812] Update Dialogue
  (bind _asbp_third_person_character (Utilities|Casting|CastToBP_ThirdPersonCharacter (Game|GetPlayerCharacter 0)))
  (Variables|/Game/ThirdPerson/Blueprints/BP_ThirdPersonCharacter.BP_ThirdPersonCharacter_C|SetCurrentDialogueText _asbp_third_person_character (Utilities|Array|Get(acopy) (Variables|Default|GetDialogue) (Variables|Default|GetCurrentDialogue)))
  (Variables|Default|SetCurrentDialogue (+ (Variables|Default|GetCurrentDialogue) 1)))

(event Custom|ResetDialogue
  ;[0.0625 0.0625 0.0625] Reset Dialogue
  (Variables|Default|SetCurrentDialogue 8)
  (CallFunction|UpdateDialogue))

(event EventBeginPlay)

(event Collision|EventActorBeginOverlap
  (params (OtherActor :type Actor%20Object%20Reference))
  ;[0.04688 0.04688 0.04688] Begin Overlap
  (if (Actor|ActorHasTag OtherActor "Player")
    (Variables|Default|SetInRange true)
    (bind _returnvalue (Actor|GetActorOfClass "/Game/ThirdPerson/Blueprints/BP_ThirdPersonCharacter.BP_ThirdPersonCharacter_C"))
    (Default|DialogueHUD _returnvalue)))

(event EventTick
  (params (DeltaSeconds :type Float%20%28single-precision%29)))

(event Collision|EventActorEndOverlap
  (params (OtherActor :type Actor%20Object%20Reference))
  ;[0.07812 0.07812 0.07812] End Overlap
  (if (Actor|ActorHasTag OtherActor "Player")
    (Variables|Default|SetInRange false)
    (Default|DeleteDialogue (stale Collision|EventActorBeginOverlap _returnvalue))))

(fn ConstructionScript)