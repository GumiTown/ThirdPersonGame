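; Enemy turret that shoots BP_EnemyBullet projectiles while an actor tagged Player overlaps it.
; Overlap events set the in-range flag; Tick then optionally rotates the turret smoothly toward the player and, after a short delay, starts firing.
; Shoot and ScatterShot re-call themselves at the firing rate while in range, the latter spawning three bullets with random yaw spread.
; VerticalFiring scales both Z values in the look-at calculation to control vertical aim.
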(event Custom|FollowPlayer
  (bind _returnvalue (Game|Player|GetPlayerPawn 0))
  (bind _returnvalue_2 (Transformation|GetActorLocation))
  (bind _returnvalue_3 (Transformation|GetActorLocation _returnvalue))
  ;[1 1 1] Follow Player
  (if (Variables|Default|GetLookAtPlayer)
    (Transformation|SetActorRotation (Math|Interpolation|RInterpTo (Transformation|GetActorRotation) (Math|Rotator|FindLookatRotation (Math|Vector|MakeVector (.x _returnvalue_2) (.y _returnvalue_2) (* (.z _returnvalue_2) (Variables|Default|GetVerticalFiring))) (Math|Vector|MakeVector (.x _returnvalue_3) (.y _returnvalue_3) (* (.z _returnvalue_3) (Variables|Default|GetVerticalFiring)))) (Utilities|Time|GetWorldDeltaSeconds) 7.0))))

(event Custom|Shoot
  (bind _sm_firingpoint (Variables|Default|GetSM_FiringPoint))
  (bind _returnvalue (Transformation|GetSocketTransform _sm_firingpoint "None" "RTS_World"))
  ;[1 1 1] Shoot
  (if (Variables|Default|GetInRange)
    (Variables|Default|SetIsShooting true)
    (Game|SpawnActorfromClass "/Game/_MyContent/BP_EnemyBullet.BP_EnemyBullet_C" (Math|Transform|MakeTransform (.location _returnvalue) (.rotation _returnvalue) "1.000000,1.000000,1.000000") "Undefined" "MultiplyWithRoot" 0 0)
    (Utilities|FlowControl|Delay (Variables|Default|GetFiringRate))
    (CallFunction|Shoot)))

(event Custom|ScatterShot
  (bind _sm_firingpoint (Variables|Default|GetSM_FiringPoint))
  (bind _returnvalue (Transformation|GetSocketTransform _sm_firingpoint "None" "RTS_World"))
  ;[1 1 1] Scatter Shot
  (if (Variables|Default|GetInRange)
    (for _index (range 0 2)
      (Variables|Default|SetIsShooting true)
      (Game|SpawnActorfromClass "/Game/_MyContent/BP_EnemyBullet.BP_EnemyBullet_C" (Math|Transform|MakeTransform (.location _returnvalue) (Math|Rotator|MakeRotator (.roll (.rotation _returnvalue)) (.pitch (.rotation _returnvalue)) (+ (.yaw (.rotation _returnvalue)) (Math|Random|RandomFloatinRange -3e+01 3e+01))) "1.000000,1.000000,1.000000") "Undefined" "MultiplyWithRoot" 0 0))
    (Utilities|FlowControl|Delay (Variables|Default|GetFiringRate))
    (CallFunction|ScatterShot)))

(event EventBeginPlay)

(event Collision|EventActorBeginOverlap
  (params (OtherActor :type Actor%20Object%20Reference))
  (if (Actor|ActorHasTag OtherActor "Player")
    (Variables|Default|SetInRange true)))

(event EventTick
  (params (DeltaSeconds :type Float%20%28single-precision%29))
  (if (Variables|Default|GetInRange)
    (CallFunction|FollowPlayer)
    (if (not (Variables|Default|GetIsShooting))
      (Utilities|FlowControl|Delay 0.5)
      (if (Variables|Default|GetIsScatterShot)
        (CallFunction|ScatterShot)
        (else
          (CallFunction|Shoot))))))

(event Collision|EventActorEndOverlap
  (params (OtherActor :type Actor%20Object%20Reference))
  (if (Actor|ActorHasTag OtherActor "Player")
    (Variables|Default|SetInRange false)
    (Variables|Default|SetIsShooting false)))

(fn ConstructionScript)