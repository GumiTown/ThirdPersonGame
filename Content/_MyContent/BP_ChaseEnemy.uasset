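; BP_ChaseEnemy is an enemy that chases the player and loses health when the player touches it.
; Tick compares player distance to the PawnSensing SightRadius, using only that radius rather than sensing events.
; In range, FollowPlayer adds movement input toward the player and smoothly interpolates rotation to face them using X and Y.
; Overlapping BP_ThirdPersonCharacter launches that character along LaunchDirection, decrements enemy Health and destroys the enemy at zero.
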(event Custom|FollowPlayer
  (bind _returnvalue (Transformation|GetActorLocation))
  (bind _returnvalue_2 (Game|Player|GetPlayerPawn 0))
  (bind _returnvalue_3 (Transformation|GetActorLocation _returnvalue_2))
  ;[1 1 1] Follow Player
  (Pawn|Input|AddMovementInput (Math|Vector|Normalize (- (Transformation|GetActorLocation (Game|Player|GetPlayerPawn 0)) (Transformation|GetActorLocation))) 1.0 false)
  (Transformation|SetActorRotation (Math|Interpolation|RInterpTo (Transformation|GetActorRotation) (Math|Rotator|FindLookatRotation (Math|Vector|MakeVector (.x _returnvalue) (.y _returnvalue) 0.0) (Math|Vector|MakeVector (.x _returnvalue_3) (.y _returnvalue_3) 0.0)) (Utilities|Time|GetWorldDeltaSeconds) 5.0)))

(event EventBeginPlay)

(event EventTick
  (params (DeltaSeconds :type Float%20%28single-precision%29))
  (if (<= (Math|Vector|Distance(Vector) (Transformation|GetActorLocation) (Transformation|GetActorLocation (Game|GetPlayerCharacter 0))) (Variables|/Script/AIModule.PawnSensingComponent|GetSightRadius (Variables|Default|GetPawnSensing)))
    (Variables|Default|SetSeesPawn true)
    (if (Variables|Default|GetSeesPawn)
      (CallFunction|FollowPlayer))))

(event Collision|EventActorBeginOverlap
  (params (OtherActor :type Actor%20Object%20Reference))
  ;[1 1 1] Damage
  (bind _asbp_third_person_character (Utilities|Casting|CastToBP_ThirdPersonCharacter OtherActor))
  (Character|LaunchCharacter _asbp_third_person_character (Variables|Default|GetLaunchDirection) false false)
  (Variables|Default|SetHealth (+ (Variables|Default|GetHealth) -1))
  (if (<= (Variables|Default|GetHealth) 0)
    (Actor|DestroyActor)))

(fn ConstructionScript)