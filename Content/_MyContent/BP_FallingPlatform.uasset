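; BP_FallingPlatform is a platform that disappears after the third-person character stands on it for a time limit, then returns.
; Overlap events set a player flag and reset the timer, which Tick increments while the flag is set.
; At the limit, the mesh is hidden with collision disabled, then restored after a respawn delay.
; PlatformShake is an unfinished custom event that only resets the mesh's relative location on alternate calls.
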(event OnComponentBeginOverlap(OverlapCollision)
  (params (OverlappedComponent :type Primitive%20Component%20Object%20Reference) (OtherActor :type Actor%20Object%20Reference) (OtherComp :type Primitive%20Component%20Object%20Reference) (OtherBodyIndex :type Integer) (bFromSweep :type Boolean) (SweepResult :type Hit%20Result%20Structure%20%28by%20ref%29))
  (Utilities|Casting|CastToBP_ThirdPersonCharacter OtherActor)
  (Development|PrintString "On Platform")
  (Variables|Default|SetPlayerOnPlatform true)
  (Variables|Default|SetTimeOnPlatform 0.0))

(event OnComponentEndOverlap(OverlapCollision)
  (params (OverlappedComponent :type Primitive%20Component%20Object%20Reference) (OtherActor :type Actor%20Object%20Reference) (OtherComp :type Primitive%20Component%20Object%20Reference) (OtherBodyIndex :type Integer))
  (Utilities|Casting|CastToBP_ThirdPersonCharacter OtherActor)
  (Variables|Default|SetPlayerOnPlatform false)
  (Variables|Default|SetTimeOnPlatform 0.0))

(event Custom|PlatformShake
  (bind _isa (Utilities|FlowControl|FlipFlop)
    (:A
      (Transformation|SetRelativeLocation (Variables|Default|GetSM_Platform) "0, 0, 0" true true))))

(event EventTick
  (params (DeltaSeconds :type Float%20%28single-precision%29))
  (if (Variables|Default|GetPlayerOnPlatform)
    (Variables|Default|SetTimeOnPlatform (+ DeltaSeconds (Variables|Default|GetTimeOnPlatform)))
    (if (>= (Variables|Default|GetTimeOnPlatform) (Variables|Default|GetTimeLimit))
      (Rendering|SetVisibility (Variables|Default|GetSM_Platform) false true)
      (Collision|SetCollisionEnabled (Variables|Default|GetSM_Platform) "NoCollision")
      (Utilities|FlowControl|Delay (Variables|Default|GetRespawnDelay))
      (Rendering|SetVisibility (Variables|Default|GetSM_Platform) true false)
      (Collision|SetCollisionEnabled (Variables|Default|GetSM_Platform) "QueryAndPhysics"))))

(fn ConstructionScript)